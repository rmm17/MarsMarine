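; BP_HealthPickup is a pickup actor that restores health to the player's BP_Marine.
; On overlap it responds only to the first player's character, and only when that marine's health is not full.
; It adds HealthToAdd, reports its AssociatedSpawnPoint to BP_MarsMarineGameMode through RegisterHealthPicked, then destroys itself.
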(event `self.ReceiveActorBeginOverlap`
  (params (OtherActor :type "Actor Object Reference"))
  (bind _returnvalue (`GameplayStatics.GetPlayerCharacter` 0))
  (if (== OtherActor _returnvalue)
    (bind _asbp_marine (cast `/Game/Blueprints/Pawns/BP_Marine` _returnvalue))
    (if (not (`/Game/Blueprints/Pawns/BP_Marine.IsHealthFull` _asbp_marine))
      (`/Game/Blueprints/Pawns/BP_Marine.AddHealth` _asbp_marine (`self.Health To Add`))
      (bind _asbp_mars_marine_game_mode (cast `/Game/Blueprints/GameModes/BP_MarsMarineGameMode` (`GameplayStatics.GetGameMode`)))
      (`/Game/Blueprints/GameModes/BP_MarsMarineGameMode.RegisterHealthPicked` _asbp_mars_marine_game_mode (`self.AssociatedSpawnPoint`))
      (`self.K2_DestroyActor`))))

(fn `UserConstructionScript`)