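; Game mode for Mars Marine that runs endless, escalating alien waves and spawns health pickups.
; Each wave scales the alien count and health spawn interval by multipliers, then looping timers spawn actors at random spawn points.
; Registered alien deaths start the next wave after a delay once none remain alive or pending.
; A map from spawn point to pickup prevents stacking, and collecting a pickup restarts the health timer.
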(event `self.ReceiveBeginPlay`
  (`KismetSystemLibrary.Delay` 2.0)
  (`self.SetupNewWave`))

(event `Event SpawnWave`
  (`self.SpawnAlien`))

(event `Event EndWave`
  (`KismetSystemLibrary.Delay` 2.0)
  (`self.SetupNewWave`))

(event `Event SpawnHealth`
  (`self.SpawnHealth`))

(fn `ClearHealthSpawnTimer`
  (`KismetSystemLibrary.K2_ClearTimer` null "Event SpawnHealth"))

(fn `GetRandomAlienSpawnPoint`
  (returns (`Spawn Point` :type "/Game/Blueprints/Actors/BP_AlienSpawnPoint Object Reference"))
  (bind _outactors (`GameplayStatics.GetAllActorsOfClass` "/Game/Blueprints/Actors/BP_AlienSpawnPoint.BP_AlienSpawnPoint_C"))
  (return (`|GetArrayItem` _outactors (`KismetMathLibrary.RandomIntegerInRange` 0 (`KismetArrayLibrary.Array_LastIndex` _outactors)))))

(fn `GetRandomHealthSpawnPoint`
  (returns (`Spawn Point` :type "/Game/Blueprints/Actors/BP_HealthSpawnPoint Object Reference"))
  (locals (UnusedSpawnPoints :type "Array of /Game/Blueprints/Actors/BP_HealthSpawnPoint Object Reference") (AllSpawnPoints :type "Array of /Game/Blueprints/Actors/BP_HealthSpawnPoint Object Reference") (UsedSpawnPoints :type "Array of /Game/Blueprints/Actors/BP_HealthSpawnPoint Object Reference"))
  (bind _unusedspawnpoints (`local.UnusedSpawnPoints`))
  (bind _outactors (`GameplayStatics.GetAllActorsOfClass` "/Game/Blueprints/Actors/BP_HealthSpawnPoint.BP_HealthSpawnPoint_C"))
  (set `local.AllSpawnPoints` _outactors)
  (`BlueprintMapLibrary.Map_Keys` (`self.HealthPickups`))
  (for _array_element (`local.AllSpawnPoints`)
    (if (not (`BlueprintMapLibrary.Map_Contains` (`self.HealthPickups`) _array_element))
      (`KismetArrayLibrary.Array_Add` (`local.UnusedSpawnPoints`) _array_element)))
  (if (not (> (`KismetArrayLibrary.Array_Length` _unusedspawnpoints) 0))
    (`self.ClearHealthSpawnTimer`))
  (return (`KismetArrayLibrary.Array_Random` _unusedspawnpoints)))

(fn `IncreaseWaveDifficulty`
  (bind _output_get (set `self.WaveDifficulty` (`KismetMathLibrary.Round` (* (`self.WaveDifficulty`) (`self.WaveDifficultyMultiplier`)))))
  (set `self.AlienSpawnsRemaining` _output_get)
  (set `self.HealthSpawnFrequency` (* (`self.HealthSpawnFrequency`) (`self.HealthDifficultyMultiplier`))))

(fn `IsWaveComplete`
  (returns (ReturnValue :type Boolean))
  (return (and (== (`KismetArrayLibrary.Array_Length` (`self.Aliens`)) 0) (== (`self.AlienSpawnsRemaining`) 0))))

(fn `RegisterAlienDeath`
  (params (Alien :type "/Game/Blueprints/Pawns/BP_Alien Object Reference"))
  (`KismetArrayLibrary.Array_RemoveItem` (`self.Aliens`) Alien)
  (if (`self.IsWaveComplete`)
    (`self.Event EndWave`)))

(fn `RegisterHealthPicked`
  (params (HealthSpawnPoint :type "/Game/Blueprints/Actors/BP_HealthSpawnPoint Object Reference"))
  (`BlueprintMapLibrary.Map_Remove` (`self.HealthPickups`) HealthSpawnPoint)
  (if true
    (`self.StartHealthSpawnTimer`)))

(fn `SetupNewWave`
  (`/Engine/EditorBlueprintResources/StandardMacros.IncrementInt` (`self.CurrentWave`)
    (:`  `
      (`self.IncreaseWaveDifficulty`)
      (`KismetSystemLibrary.K2_SetTimer` null "Event SpawnWave" (`self.AlienSpawnFrequency`) true)
      (`self.StartHealthSpawnTimer`))))

(fn `SpawnAlien`
  (bind _spawn_point (`self.GetRandomAlienSpawnPoint`))
  (`/Engine/EditorBlueprintResources/StandardMacros.IsValid` _spawn_point
    (:`Is Valid`
      (bind _returnvalue (`|SpawnActorFromClass` "/Game/Blueprints/Pawns/BP_Alien.BP_Alien_C" (`self.GetTransform` _spawn_point) "Undefined" "OverrideRootScale" null null))
      (`/Engine/EditorBlueprintResources/StandardMacros.IsValid` _returnvalue
        (:`Is Valid`
          (`KismetArrayLibrary.Array_Add` (`self.Aliens`) _returnvalue)
          (bind _result (`/Engine/EditorBlueprintResources/StandardMacros.DecrementInt` (`self.AlienSpawnsRemaining`))
            (:`  `
              (if (== _result 0)
                (`KismetSystemLibrary.K2_ClearTimer` null "Event SpawnWave")))))))))

(fn `SpawnHealth`
  (locals (SpawnPoint :type "/Game/Blueprints/Actors/BP_HealthSpawnPoint Object Reference"))
  (bind _spawn_point (`self.GetRandomHealthSpawnPoint`))
  (`/Engine/EditorBlueprintResources/StandardMacros.IsValid` _spawn_point
    (:`Is Valid`
      (set `local.SpawnPoint` _spawn_point)
      (bind _keys (`BlueprintMapLibrary.Map_Keys` (`self.HealthPickups`)))
      (if (not (`KismetArrayLibrary.Array_Contains` _keys (`local.SpawnPoint`)))
        (bind _returnvalue (`|SpawnActorFromClass` "/Game/Blueprints/Actors/BP_HealthPickup.BP_HealthPickup_C" (`self.GetTransform` (`local.SpawnPoint`)) "Undefined" "OverrideRootScale" null null))
        (`/Engine/EditorBlueprintResources/StandardMacros.IsValid` _returnvalue
          (:`Is Valid`
            (`BlueprintMapLibrary.Map_Add` (`self.HealthPickups`) (`local.SpawnPoint`) _returnvalue)
            (set `/Game/Blueprints/Actors/BP_HealthPickup.AssociatedSpawnPoint` (`local.SpawnPoint`) _returnvalue)))))))

(fn `StartHealthSpawnTimer`
  (if (`KismetSystemLibrary.K2_IsTimerActive` null "Event SpawnHealth")
    (`KismetSystemLibrary.K2_ClearTimer` null "Event SpawnHealth"))
  (`KismetSystemLibrary.K2_SetTimer` null "Event SpawnHealth" (`self.HealthSpawnFrequency`) true))

(fn `UserConstructionScript`)